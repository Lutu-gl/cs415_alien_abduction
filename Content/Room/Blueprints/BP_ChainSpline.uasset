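; Construction-script Blueprint that builds a chain of static mesh links along an editable spline.
; It divides the spline length by Spacing and places a ChainMesh component at each step, aligned to the spline's local rotation and scaled by ChainSize.
; A second link sits halfway between each step with ChainAngle added to its roll, producing the alternating interlocked look of a chain.
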(fn ConstructionScript
  (for _index (range 1 (.ReturnValue (Math|Float|Division(WholeandRemainder) (Spline|GetSplineLength (Variables|Default|GetSpline)) (Variables|Default|GetSpacing))))
    (bind _returnvalue (AddComponent|AddStaticMeshComponent false (Math|Transform|MakeTransform (Spline|GetLocationatDistanceAlongSpline (Variables|Default|GetSpline) (* _index (Variables|Default|GetSpacing)) "Local") (Spline|GetRotationatDistanceAlongSpline (Variables|Default|GetSpline) (* _index (Variables|Default|GetSpacing)) "Local") (Variables|Default|GetChainSize))))
    (Components|StaticMesh|SetStaticMesh _returnvalue (Variables|Default|GetChainMesh))
    (bind _returnvalue_2 (AddComponent|AddStaticMeshComponent false (Math|Transform|MakeTransform (Spline|GetLocationatDistanceAlongSpline (Variables|Default|GetSpline) (- (* _index (Variables|Default|GetSpacing)) (/ (Variables|Default|GetSpacing) 2.0)) "Local") (Math|Rotator|MakeRotator (+ (.Roll (Math|Rotator|BreakRotator (Spline|GetRotationatDistanceAlongSpline (Variables|Default|GetSpline) (- (* _index (Variables|Default|GetSpacing)) (/ (Variables|Default|GetSpacing) 2.0)) "Local"))) (Variables|Default|GetChainAngle)) (.Pitch (Math|Rotator|BreakRotator (Spline|GetRotationatDistanceAlongSpline (Variables|Default|GetSpline) (- (* _index (Variables|Default|GetSpacing)) (/ (Variables|Default|GetSpacing) 2.0)) "Local"))) (.Yaw (Math|Rotator|BreakRotator (Spline|GetRotationatDistanceAlongSpline (Variables|Default|GetSpline) (- (* _index (Variables|Default|GetSpacing)) (/ (Variables|Default|GetSpacing) 2.0)) "Local")))) (Variables|Default|GetChainSize))))
    (Components|StaticMesh|SetStaticMesh _returnvalue_2 (Variables|Default|GetChainMesh))))