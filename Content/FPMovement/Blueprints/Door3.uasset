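; Door3 is a locked exit door that sends the player on to the Room4 level.
; When its Box is overlapped, it casts the other actor to BP_Player and opens the level by name only if HasKey3 is true.
; Disconnected, unused nodes remain for a GameDone end screen with game pause, and for destroying the player.
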(event OnComponentBeginOverlap(Box)
  (params (OverlappedComponent :type Primitive%20Component%20Object%20Reference) (OtherActor :type Actor%20Object%20Reference) (OtherComp :type Primitive%20Component%20Object%20Reference) (OtherBodyIndex :type Integer) (bFromSweep :type Boolean) (SweepResult :type Hit%20Result%20Structure%20%28by%20ref%29))
  (bind _asbp_player (Utilities|Casting|CastToBP_Player OtherActor))
  (if (Variables|/Game/FPMovement/Player/Blueprints/BP_Player.BP_Player_C|GethasKey3 _asbp_player)
    (Game|OpenLevel(byName) "Room4")))

(event EventBeginPlay)

(event Collision|EventActorBeginOverlap
  (params (OtherActor :type Actor%20Object%20Reference)))

(event EventTick
  (params (DeltaSeconds :type Float%20%28single-precision%29)))

(fn ConstructionScript)