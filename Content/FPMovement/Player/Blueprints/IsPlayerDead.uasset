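; IsPlayerDead is an actor that watches for the player's death and triggers the game over screen.
; Every Tick it casts player pawn 0 to BP_Player and checks whether Health equals exactly zero.
; On a match it adds the GameOver widget to the viewport, shows the cursor, switches to UI-only input, pauses the game and destroys the player.
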(event EventBeginPlay)

(event Collision|EventActorBeginOverlap
  (params (OtherActor :type Actor%20Object%20Reference)))

(event EventTick
  (params (DeltaSeconds :type Float%20%28single-precision%29))
  (bind _returnvalue (Game|GetPlayerController 0))
  (bind _asbp_player (Utilities|Casting|CastToBP_Player (Game|Player|GetPlayerPawn 0)))
  (if (== (Variables|/Game/FPMovement/Player/Blueprints/BP_Player.BP_Player_C|GetHealth _asbp_player) 0)
    (bind _returnvalue_2 (UserInterface|CreateWidget "/Game/FPMovement/UI/GameOver.GameOver_C"))
    (UserInterface|Viewport|AddtoViewport _returnvalue_2 0)
    (Variables|/Script/Engine.PlayerController|SetbShowMouseCursor _returnvalue true)
    (Input|SetInputModeUIOnly _returnvalue 0 "DoNotLock" true)
    (Game|SetGamePaused true)
    (Actor|DestroyActor _asbp_player)))

(fn ConstructionScript)